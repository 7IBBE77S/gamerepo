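; A wandering animal character, named as an inventory item, that can be captured to follow the player.
; From BeginPlay it repeatedly moves to random reachable points nearby, pausing after each successful move.
; Capture halts movement and starts a similar AIMoveTo loop toward the player; both loops re-arm only on success.
; PickUpItem prints a debug message and returns its Item; the destroy event and Wander2 are empty stubs.
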(event Custom|Destroy%20itwem)

(event Custom|Wonder
  (AI|AIMoveTo self (.RandomLocation (AI|Navigation|GetRandomReachablePointinRadius (Transformation|GetActorLocation) 5e+02 0 0)) 0 12.0 false
    (:OnSuccess
      (Utilities|FlowControl|Delay 2.0)
      (CallFunction|Wonder))))

(event Custom|Follow%20Player
  (AI|AIMoveTo self "0, 0, 0" (Game|GetPlayerCharacter 0) 2e+02 false
    (:OnSuccess
      (Utilities|FlowControl|Delay 0.5)
      (CallFunction|FollowPlayer))))

(event EventBeginPlay
  (CallFunction|Wonder))

(event EventCapture
  (Components|Movement|StopMovementImmediately (Variables|Character|GetCharacterMovement))
  (CallFunction|FollowPlayer))

(fn ConstructionScript)

(fn Wander2)

(fn PickUpItem
  (Development|PrintString "animal picked")
  (return (Variables|Default|Getitem)))